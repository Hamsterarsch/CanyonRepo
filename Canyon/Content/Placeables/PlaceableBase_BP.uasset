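; PlaceableBase_BP is, by its name, a base actor for placeable objects, providing influence-type queries and a selection highlight.
; Getter functions expose its InfluenceType as an integer and return the InfluenceTypes enum class.
; Two near-identical toggle functions flip IsHighlighted, showing MPMeshCollisionComp with a selection material when on and hiding it when off.
; The event graph and construction script contain no logic.
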(event EventBeginPlay)

(event Collision|EventActorBeginOverlap
  (params (OtherActor :type Actor%20Object%20Reference)))

(event EventTick
  (params (DeltaSeconds :type Float%20%28single-precision%29)))

(fn ConstructionScript)

(fn GetInfluenceEnumValue
  (return (Math|Conversions|ToInteger(Byte) (Variables|Default|GetInfluenceType))))

(fn GetInfluenceEnumClass
  (return "/Game/Placeables/InfluenceTypes.InfluenceTypes"))

(fn ToggleSelectionHighlight
  (bind _output_get (Variables|Default|SetbIsHighlighted (not (Variables|Default|GetbIsHighlighted))))
  (if _output_get
    (Rendering|SetVisibility (Variables|Default|Getm_pMeshCollisionComp) true false)
    (Rendering|Material|SetMaterial (Variables|Default|Getm_pMeshCollisionComp) 0 "/Game/ArtAssets/PlaceableSelection_M.PlaceableSelection_M")
    (else
      (Rendering|SetVisibility (Variables|Default|Getm_pMeshCollisionComp) false false)))
  (return _output_get false))

(fn OnToggleSelectionHighlight
  (bind _output_get (Variables|Default|SetbIsHighlighted (not (Variables|Default|GetbIsHighlighted))))
  (if _output_get
    (Rendering|SetVisibility (Variables|Default|Getm_pMeshCollisionComp) true false)
    (Rendering|Material|SetMaterial (Variables|Default|Getm_pMeshCollisionComp) 0 "/Game/ArtAssets/PlaceableSelection_M.PlaceableSelection_M")
    (else
      (Rendering|SetVisibility (Variables|Default|Getm_pMeshCollisionComp) false false)))
  (return _output_get))