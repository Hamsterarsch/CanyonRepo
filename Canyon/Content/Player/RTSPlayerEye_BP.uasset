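; RTS player eye Blueprint that serves as the Wwise audio listener and plays building placement feedback sounds.
; It registers itself as default listener, then each tick updates its transform and sets wind and music lowpass RTPCs from camera height relative to max zoom.
; Preview events start and stop the placement sound, with commit also playing a large or small score-up or score-down effect based on point delta.
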(event EventBeginPlay
  (Class|AkGameplayStatics|RegisterDefaultListener self))

(event Collision|EventActorBeginOverlap
  (params (OtherActor :type Actor%20Object%20Reference)))

(event EventTick
  (params (DeltaSeconds :type Float%20%28single-precision%29))
  (bind _returnvalue (Class|RTSPlayerEye|GetMaxZoomDist))
  (bind _m_pcamera (Variables|Default|Getm_pCamera))
  (bind _returnvalue_2 (Transformation|GetWorldLocation _m_pcamera))
  (bind _returnvalue_3 (- _returnvalue 1.0))
  (bind _z (Math|Vector|BreakVector _returnvalue_2))
  (bind _returnvalue_4 (/ _z _returnvalue_3))
  (Class|AkGameplayStatics|SetObjectTransform self (Transformation|GetActorLocation) (Transformation|GetActorForwardVector) (Transformation|GetActorUpVector))
  (Class|AkGameplayStatics|SetRTPCValue "VolumeCoeffWind" _returnvalue_4)
  (Class|AkGameplayStatics|SetRTPCValue "LowpassCoeffMusic" _returnvalue_4))

(event EventOnCommitPreviewBuilding
  (params (PointDelta :type Integer))
  (Class|AkGameplayStatics|PostEvent "/Game/wwise/assets/DeactivateEffectBuildingInPlacement.DeactivateEffectBuildingInPlacement" self)
  (if (> PointDelta 50)
    (Class|AkGameplayStatics|PostEvent "/Game/wwise/assets/PlayEffectScoreUpLarge.PlayEffectScoreUpLarge" self)
    (elif (< PointDelta -50)
      (Class|AkGameplayStatics|PostEvent "/Game/wwise/assets/PlayEffectScoreDownLarge.PlayEffectScoreDownLarge" self)
      (elif (>= PointDelta 0)
        (Class|AkGameplayStatics|PostEvent "/Game/wwise/assets/PlayEffectScoreUpSmall.PlayEffectScoreUpSmall" self)
        (else
          (Class|AkGameplayStatics|PostEvent "/Game/wwise/assets/PlayEffectScoreDownSmall.PlayEffectScoreDownSmall" self))))))

(event EventOnBeginPreviewBuilding
  (Class|AkGameplayStatics|PostEvent "/Game/wwise/assets/ActivateEffectBuildingInPlacement.ActivateEffectBuildingInPlacement" self))

(event EventOnAbortPreviewBuilding
  (Class|AkGameplayStatics|PostEvent "/Game/wwise/assets/DeactivateEffectBuildingInPlacement.DeactivateEffectBuildingInPlacement" self))

(fn ConstructionScript)