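; Game instance Blueprint for the Canyon game that owns the loading screen and sets starting audio volumes.
; On Init it creates the LoadingScreen widget once and adds it to the viewport at a raised Z-order.
; Begin and end loading events show or hide that persistent widget.
; Init also sets the Wwise RTPC volume coefficients for master, effects, music and voice to half as fixed defaults.
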(event EventOnEndLoadingScreen
  (params (pLoadedWorld :type World%20Object%20Reference))
  (Class|PrettyWidget|HideWidget (Variables|Default|GetLoadingScreen)))

(event EventOnBeginLoadingScreen
  (params (MapName :type String))
  (Class|PrettyWidget|ShowWidget (Variables|Default|GetLoadingScreen)))

(event EventInit
  (bind _returnvalue (UserInterface|CreateWidget "/Game/Widgets/Menu/LoadingScreen.LoadingScreen_C"))
  (bind _output_get (Variables|Default|SetLoadingScreen _returnvalue))
  (UserInterface|Viewport|AddtoViewport _output_get 10)
  (CallFunction|InitWWiseBusVolumes))

(fn InitWWiseBusVolumes
  (Class|AkGameplayStatics|SetRTPCValue "VolumeCoeffMaster" 0.5)
  (Class|AkGameplayStatics|SetRTPCValue "VolumeCoeffEffects" 0.5)
  (Class|AkGameplayStatics|SetRTPCValue "VolumeCoeffMusic" 0.5)
  (Class|AkGameplayStatics|SetRTPCValue "VolumeCoeffVoice" 0.5))