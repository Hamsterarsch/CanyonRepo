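; Default game mode Blueprint for Canyon that handles the startup wind audio and the new-deck popup.
; On BeginPlay it posts the ActivateWindZoom Wwise event on itself and adds a collapsed PopupDeck widget to the viewport.
; The new-deck notification shows that widget without blocking input, then calls its hide after a two-second delay.
; The lose and next-level notifications are empty stubs.
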(event EventBeginPlay
  (Class|AkGameplayStatics|PostEvent "/Game/wwise/assets/ActivateWindZoom.ActivateWindZoom" self)
  (bind _returnvalue (UserInterface|CreateWidget "/Game/Widgets/Popups/PopupDeck.PopupDeck_C"))
  (bind _output_get (Variables|Default|SetPopupDeck _returnvalue))
  (Widget|SetVisibility _output_get "Collapsed")
  (UserInterface|Viewport|AddtoViewport _output_get 0))

(event EventTick
  (params (DeltaSeconds :type Float%20%28single-precision%29)))

(event EventNotifyonNewDeckAvailable
  (bind _popupdeck (Variables|Default|GetPopupDeck))
  (Widget|SetVisibility _popupdeck "HitTestInvisible")
  (Class|PrettyWidget|ShowWidget _popupdeck)
  (Utilities|FlowControl|Delay 2.0)
  (Class|PrettyWidget|HideWidget _popupdeck))

(event EventNotifyonLoose)

(event EventNotifyNextLevelAvailable)

(fn ConstructionScript)