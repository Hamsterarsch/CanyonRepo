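; InfluenceFloatMapDAL_BP is an accessor that exposes a map keyed by the InfluenceTypes enum through string category names.
; GetValueForCategory converts a name to its enum entry and returns the mapped value as a float, or -1 when the key is missing.
; GetMap copies every entry into LocalProbMap, with enum keys converted to strings, and returns that map.
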(fn GetValueforCategory
  (params (CategoryName :type String))
  (bind _returnvalue (Class|CanyonBpfLib|EnumStringtoEnumByte "/Game/Placeables/InfluenceTypes.InfluenceTypes" CategoryName))
  (bind _mapping (Variables|Default|GetMapping))
  (bind _returnvalue_2 (Utilities|Enum|ByteToEnumInfluenceTypes _returnvalue))
  (bind (_value _returnvalue_3) (Utilities|Map|Find _mapping _returnvalue_2))
  (if _returnvalue_3
    (return (Math|Conversions|ToFloat(Integer) _value))
    (else
      (return -1.0))))

(fn GetMap
  (bind _mapping (Variables|Default|GetMapping))
  (bind _keys (Utilities|Map|Keys _mapping))
  (bind _values (Utilities|Map|Values _mapping))
  (for (_array_element _array_index) _keys
    (Utilities|Map|Add (LocalVariables|GetLocalProbMap) (Utilities|String|EnumtoString _array_element) (Utilities|Array|Get(acopy) _values _array_index)))
  (return (LocalVariables|GetLocalProbMap)))